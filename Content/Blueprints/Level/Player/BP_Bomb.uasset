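; Bomb actor Blueprint that handles the audio and visual feedback of a placed bomb, from placement through warning to explosion.
; On BeginPlay it plays a placement sound, and the authority triggers a looping warning animation and sound after a delay.
; The bound OnBombExploded event destroys the mesh, plays the blast sound and shakes cameras.
; The shake epicenter is offset from the camera so falloff follows the view target's distance to the bomb.
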(event Custom|OnBombExploded_Event_0
  (CallFunction|PlayExplosionSound))

(event Custom|OnBombWarning
  (bind _meshcomponent (Variables|Default|GetMeshComponent))
  (Utilities|IsValid _meshcomponent
    (:Is%20Valid
      (Components|Animation|PlayAnimation _meshcomponent "/Game/Materials/Bomb/A_BombWarning.A_BombWarning" true)
      (Audio|PlaySoundatLocation "/Game/Sounds/SC_BombWarning.SC_BombWarning" (Transformation|GetActorLocation) "0, 0, 0" 1.0 1.0 0.0 0 0 0 0))))

(event Custom|PlayExplosionSound
  (bind _returnvalue (Transformation|GetActorLocation))
  (bind _meshcomponent (Variables|Default|GetMeshComponent))
  (Utilities|IsValid _meshcomponent
    (:Is%20Valid
      (Components|DestroyComponent _meshcomponent))
    (:Is%20Not%20Valid
      _))
  (Camera|PlayWorldCameraShake "/Game/Blueprints/Level/Player/BP_CameraShake.BP_CameraShake_C" (+ (- (Transformation|GetActorLocation (Pawn|GetViewTarget (Game|GetPlayerController 0))) _returnvalue) (Camera|GetCameraLocation (Game|GetPlayerCameraManager 0))) 0.0 5e+02)
  (Audio|PlaySoundatLocation "/Game/Sounds/SC_BombExplosion.SC_BombExplosion" _returnvalue "0, 0, 0" 1.0 1.0 0.0 0 0 0 0))

(event EventBeginPlay
  (Audio|PlaySoundatLocation "/Game/Sounds/SC_BombPlace.SC_BombPlace" (Transformation|GetActorLocation) "0, 0, 0" 1.0 1.0 0.0 0 0 0 0)
  (EventDispatchers|AssignOnBombExploded (delegate Custom|OnBombExploded_Event_0))
  (Networking|SwitchHasAuthority
    (:Authority
      (Utilities|FlowControl|Delay 2.5)
      (CallFunction|OnBombWarning))))

(fn ConstructionScript)