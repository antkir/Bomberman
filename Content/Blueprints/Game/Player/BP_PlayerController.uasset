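; Player controller that drives the match UI and audio listener for a round-based game.
; Match-phase events create the pre-game, HUD, begin-game, round over, draw and game over widgets, clearing stale result screens at pre-game.
; A toggle event shows or hides the game menu, which game over also closes while disabling input.
; On local controllers, Tick moves the audio listener toward the view target at constant speed with fixed rotation.
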(event EventBeginPlay
  (bind _returnvalue (Pawn|GetViewTarget))
  (Utilities|IsValid _returnvalue
    (:Is%20Valid
      (Variables|Default|SetPrevViewTarget (Transformation|GetActorLocation _returnvalue)))))

(event EventTick
  (params (DeltaSeconds :type Float%20%28single-precision%29))
  (bind _returnvalue (Pawn|GetViewTarget))
  (if (Pawn|IsLocalPlayerController)
    (Utilities|IsValid _returnvalue
      (:Is%20Valid
        (bind _output_get (Variables|Default|SetPrevViewTarget (Math|Interpolation|VInterptoConstant (Variables|Default|GetPrevViewTarget) (Transformation|GetActorLocation _returnvalue) DeltaSeconds 3e+03)))
        (Class|PlayerController|SetAudioListenerOverride 0 _output_get "0,-90.000000, 0")))))

(event EventOnBeginPreGame
  (params (Countdown :type Float%20%28single-precision%29))
  (bind _gameoverwidget (Variables|Default|GetGameOverWidget))
  (bind _roundoverwidget (Variables|Default|GetRoundOverWidget))
  (bind _rounddrawwidget (Variables|Default|GetRoundDrawWidget))
  (Development|PrintString "Hello" true true "(R=0.000000,G=0.660000,B=1.000000,A=1.000000)" 1e+01)
  (Utilities|IsValid _roundoverwidget
    (:Is%20Valid
      (Widget|RemovefromParent _roundoverwidget))
    (:Is%20Not%20Valid
      _))
  (Utilities|IsValid _rounddrawwidget
    (:Is%20Valid
      (Widget|RemovefromParent _rounddrawwidget))
    (:Is%20Not%20Valid
      _))
  (Utilities|IsValid _gameoverwidget
    (:Is%20Valid
      (Widget|RemovefromParent _gameoverwidget))
    (:Is%20Not%20Valid
      _))
  (bind _returnvalue (UserInterface|CreateWidget "/Game/Blueprints/Game/UI/WBP_PreGame.WBP_PreGame_C" 0 (Math|Float|Truncate Countdown)))
  (UserInterface|Viewport|AddtoViewport _returnvalue 0)
  (Input|EnableInput 0))

(event EventOnBeginGame
  (Utilities|IsValid (Variables|Default|GetGameWidget)
    (:Is%20Valid
      _)
    (:Is%20Not%20Valid
      (bind _returnvalue (UserInterface|CreateWidget "/Game/Blueprints/Game/UI/WBP_Game.WBP_Game_C"))
      (bind _output_get (Variables|Default|SetGameWidget _returnvalue))
      (UserInterface|Viewport|AddtoViewport _output_get 0)))
  (bind _returnvalue_2 (UserInterface|CreateWidget "/Game/Blueprints/Game/UI/WBP_BeginGame.WBP_BeginGame_C"))
  (UserInterface|Viewport|AddtoViewport _returnvalue_2 0))

(event EventOnBeginRoundOver
  (params (PlayerName :type String))
  (bind _returnvalue (UserInterface|CreateWidget "/Game/Blueprints/Game/UI/WBP_RoundOver.WBP_RoundOver_C" 0 (Utilities|Text|ToText(String) PlayerName)))
  (bind _output_get (Variables|Default|SetRoundOverWidget _returnvalue))
  (UserInterface|Viewport|AddtoViewport _output_get 0))

(event EventOnBeginGameOver
  (params (PlayerName :type String))
  (bind _gamemenuwidget (Variables|Default|GetGameMenuWidget))
  (bind _returnvalue (UserInterface|CreateWidget "/Game/Blueprints/Game/UI/WBP_GameOver.WBP_GameOver_C" 0 (Utilities|Text|ToText(String) PlayerName)))
  (bind _output_get (Variables|Default|SetGameOverWidget _returnvalue))
  (UserInterface|Viewport|AddtoViewport _output_get 0)
  (Utilities|IsValid _gamemenuwidget
    (:Is%20Valid
      (Widget|RemovefromParent _gamemenuwidget)
      (Input|DisableInput 0))))

(event EventOnToggleGameMenu
  (if (Variables|Default|GetbIsGameMenuOpen)
    (bind _returnvalue (UserInterface|CreateWidget "/Game/Blueprints/Game/UI/WBP_GameMenu.WBP_GameMenu_C"))
    (bind _output_get (Variables|Default|SetGameMenuWidget _returnvalue))
    (UserInterface|Viewport|AddtoViewport _output_get 1)
    (else
      (Utilities|IsValid (Variables|Default|GetGameMenuWidget)
        (:Is%20Valid
          (Widget|RemovefromParent (Variables|Default|GetGameMenuWidget)))))))

(event EventOnBeginRoundDraw
  (bind _returnvalue (UserInterface|CreateWidget "/Game/Blueprints/Game/UI/WBP_RoundDraw.WBP_RoundDraw_C"))
  (bind _output_get (Variables|Default|SetRoundDrawWidget _returnvalue))
  (UserInterface|Viewport|AddtoViewport _output_get 0))

(fn ConstructionScript)