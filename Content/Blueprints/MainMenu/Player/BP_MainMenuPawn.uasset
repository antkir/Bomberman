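; BP_MainMenuPawn is the dancing Bomberman character shown in the main menu.
; On BeginPlay it creates a dynamic material from M_BomberMan and picks one of four player colors and looping dance animations from the game instance's SkinIndex modulo four.
; It then increments SkinIndex, so each pawn that begins play gets the next skin and dance in the cycle.
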(event EventBeginPlay
  (bind _returnvalue (Game|GetGameInstance))
  (Utilities|IsValid _returnvalue
    (:Is%20Valid
      (bind _asbp_game_instance (Utilities|Casting|CastToBP_GameInstance _returnvalue))
      (bind _returnvalue_2 (Rendering|Material|CreateDynamicMaterialInstance (Variables|Character|GetMesh) 0 "/Game/Materials/BomberMan/M_BomberMan.M_BomberMan" "None" :!class /Script/Engine.PrimitiveComponent))
      (Rendering|Material|SetVectorParameterValue _returnvalue_2 "PlayerColor" (Utilities|Select :Index (Math|Integer|%(Integer) (Variables|/Game/Blueprints/BP_GameInstance.BP_GameInstance_C|GetSkinIndex _asbp_game_instance) 4) :Option%200 "(R=1.000000,G=0.000000,B=0.000000,A=1.000000)" :Option%201 "(R=0.000000,G=1.000000,B=0.000000,A=1.000000)" :Option%202 "(R=0.000000,G=0.000000,B=1.000000,A=1.000000)" :Option%203 "(R=1.000000,G=1.000000,B=0.000000,A=1.000000)") :!class /Script/Engine.MaterialInstanceDynamic)
      (Components|Animation|PlayAnimation (Variables|Character|GetMesh) (Utilities|Select :Index (Math|Integer|%(Integer) (Variables|/Game/Blueprints/BP_GameInstance.BP_GameInstance_C|GetSkinIndex _asbp_game_instance) 4) :Option%200 "/Game/Materials/BomberMan/A_Dance1.A_Dance1" :Option%201 "/Game/Materials/BomberMan/A_Dance2.A_Dance2" :Option%202 "/Game/Materials/BomberMan/A_Dance3.A_Dance3" :Option%203 "/Game/Materials/BomberMan/A_Dance4.A_Dance4") true)
      (Variables|/Game/Blueprints/BP_GameInstance.BP_GameInstance_C|SetSkinIndex _asbp_game_instance (+ (Variables|/Game/Blueprints/BP_GameInstance.BP_GameInstance_C|GetSkinIndex _asbp_game_instance) 1)))))

(fn ConstructionScript)