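; BP_MainMenuPlayerController is the main menu player controller that puts up the menu and loading screens.
; On BeginPlay, outside dedicated servers, it creates WBP_MainMenu for player controller 0 and adds it to the viewport.
; Its OnStartGame event, on the local controller only, removes all widgets and shows WBP_Loading.
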(event Custom|On%20Start%20Game
  (if (Pawn|IsLocalController)
    (Viewport|RemoveAllWidgets)
    (bind _returnvalue (UserInterface|CreateWidget "/Game/Blueprints/MainMenu/UI/WBP_Loading.WBP_Loading_C"))
    (UserInterface|Viewport|AddtoViewport _returnvalue 0)))

(event EventBeginPlay
  (if (not (Networking|IsDedicatedServer))
    (bind _returnvalue (UserInterface|CreateWidget "/Game/Blueprints/MainMenu/UI/WBP_MainMenu.WBP_MainMenu_C" (Game|GetPlayerController 0)))
    (UserInterface|Viewport|AddtoViewport _returnvalue 0)))

(fn ConstructionScript)